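; Interactive chair in a subway train that cycles through four materials on X and logs usage data to CSV.
; Overlapping its box enables input and toggles a text prompt.
; X events also count uses, time intervals between presses and write Data.csv, combining this count with one from the SM_chair_01aBP actor.
; A looping one-second timer tracks elapsed play time in t1.csv, and BeginPlay also runs the count-and-save step.
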(event `self.BoxDesc.OnComponentBeginOverlap`
  (params (OverlappedComponent :type "PrimitiveComponent Object Reference") (OtherActor :type "Actor Object Reference") (OtherComp :type "PrimitiveComponent Object Reference") (OtherBodyIndex :type Integer) (bFromSweep :type Boolean) (SweepResult :type "HitResult Structure (by ref)"))
  (`self.EnableInput` (`GameplayStatics.GetPlayerController` 0))
  (`SceneComponent.ToggleVisibility` (`self.TEXT`) false :!label _label))

(event `self.BoxDesc.OnComponentEndOverlap`
  (params (OverlappedComponent :type "PrimitiveComponent Object Reference") (OtherActor :type "Actor Object Reference") (OtherComp :type "PrimitiveComponent Object Reference") (OtherBodyIndex :type Integer))
  (`self.DisableInput` (`GameplayStatics.GetPlayerController` 0))
  (goto _label))

(event `Key|X`
  (params (Key :type "Key Structure"))
  (bind _staticmesh (`self.StaticMesh`))
  (:`Pressed`
    (`|MultiGate` false true 0
      (:`Out 0`
        (`PrimitiveComponent.SetMaterial` _staticmesh 0 "/Game/SubwayTrain/Materials/Instances/MI_Chair_01.MI_chair_01"))
      (:`Out 1`
        (`PrimitiveComponent.SetMaterial` _staticmesh 0 "/Game/SubwayTrain/Materials/Instances/MI_Chair_02.MI_Chair_02"))
      (:`Out 2`
        (`PrimitiveComponent.SetMaterial` _staticmesh 0 "/Game/SubwayTrain/Materials/Instances/MI_Chair_03.MI_Chair_03"))
      (:`Out 3`
        (`PrimitiveComponent.SetMaterial` _staticmesh 0 "/Game/SubwayTrain/Materials/Instances/MI_Chair_04.MI_Chair_04"))))
  (:`Released`
    (set `self.CountChair2` (`KismetTextLibrary.Conv_TextToString` (`KismetTextLibrary.Conv_IntToText` (+ (`KismetStringLibrary.Conv_StringToInt` (`self.CountChair2`)) 1 0))) :!label _label_2)
    (`TextFileManager.SaveArrayText` (`KismetSystemLibrary.GetProjectDirectory`) "Data.csv" (`|MakeArray` (`self.Chairs info`) (`KismetStringLibrary.Concat_StrStr` (`KismetStringLibrary.Concat_StrStr` (`KismetStringLibrary.Concat_StrStr` (`KismetStringLibrary.Concat_StrStr` (`KismetStringLibrary.Concat_StrStr` (`KismetStringLibrary.Concat_StrStr` (`/Game/SubwayTrain/Blueprints/SM_chair_01aBP.count2` (stale `self.ReceiveBeginPlay` _returnvalue)) ",") (`self.CountChair2`)) ",") (`KismetStringLibrary.Conv_IntToString` (stale `self.ReceiveBeginPlay` _output_get))) ",") (`KismetStringLibrary.Conv_DoubleToString` (stale _output_get_4)))) true :!label _label_3)))

(event `self.ReceiveBeginPlay`
  (bind _returnvalue (`GameplayStatics.GetActorOfClass` "/Game/SubwayTrain/Blueprints/SM_chair_01aBP.SM_chair_01aBP_C"))
  (`KismetSystemLibrary.K2_SetTimer` null "increment" 1.0 true)
  (bind _output_get (set `self.value` (+ (`self.value`) 1)))
  (`KismetSystemLibrary.PrintString` (`KismetStringLibrary.Conv_IntToString` _output_get))
  (goto _label_2))

(event `Key|X`
  (params (Key :type "Key Structure"))
  (:`Pressed`
    (if (== (`self.t1`) 0.0)
      (bind _output_get (set `self.t1` (`self.GetGameTimeSinceCreation` (stale `self.ReceiveBeginPlay` _returnvalue))))
      (bind _output_get_2 (set `self.elapsedTime` _output_get))
      (`KismetSystemLibrary.PrintString` (`KismetStringLibrary.Conv_DoubleToString` _output_get_2))
      (else
        (set `self.t2` (`self.GetGameTimeSinceCreation` (stale `self.ReceiveBeginPlay` _returnvalue)))
        (bind _output_get_3 (set `self.elapsedTime` (- (`self.t2`) (`self.t1`))))
        (`KismetSystemLibrary.PrintString` (`KismetStringLibrary.Conv_DoubleToString` _output_get_3))
        (bind _output_get_4 (set `self.t1` (`self.t2`)))
        (goto _label_3)))))

(event `Key|Z`
  (params (Key :type "Key Structure")))

(event `Key|X`
  (params (Key :type "Key Structure"))
  (:`Released`
    (if (== (`self.t1`) 0.0)
      (bind _output_get (set `self.t1` (`self.GetGameTimeSinceCreation`)))
      (bind _output_get_2 (set `self.elapsedTime` _output_get))
      (`KismetSystemLibrary.PrintString` (`KismetStringLibrary.Conv_DoubleToString` _output_get_2) true true (struct :`R` 1.0 :`G` 0.184767 :`B` 0.324781 :`A` 1.0))
      (else
        (set `self.t2` (`self.GetGameTimeSinceCreation`))
        (bind _output_get_3 (set `self.elapsedTime` (- (`self.t2`) (`self.t1`))))
        (`KismetSystemLibrary.PrintString` (`KismetStringLibrary.Conv_DoubleToString` _output_get_3) true true (struct :`R` 1.0 :`G` 0.406265 :`B` 0.316457 :`A` 1.0))
        (set `self.t1` (`self.t2`))))))

(fn `increment`
  (bind _output_get (set `self.value` (+ (`self.value`) 1)))
  (bind _returnvalue (`KismetStringLibrary.Conv_IntToString` _output_get))
  (`KismetSystemLibrary.PrintString` _returnvalue)
  (`TextFileManager.SaveArrayText` (`KismetSystemLibrary.GetProjectDirectory`) "t1.csv" (`|MakeArray` (`self.Total time`) _returnvalue) true)
  (return))

(fn `UserConstructionScript`)